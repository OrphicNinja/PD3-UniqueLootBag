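; Mod actor that retextures loot bags by bag type, giving each type a unique look.
; BeginPlay builds a dynamic instance of MI_CustomBag per BagTextureMap entry into BagMIDMap, and binds to bag trigger volumes within that loop.
; Tick polls all valuable-bag and back-item actors, swapping mismatched materials.
; The entered-or-secured event reskins the secured-bag actor at SecureIndex, advancing the index only when the material changes.
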(event Custom|OnBagEnteredOrSecured_Event_0
  (params (Volume :type SBZ%20Bag%20Trigger%20Volume%20Object%20Reference) (Bag :type SBZ%20Bag%20Item%20Object%20Reference) (Handle :type SBZ%20Bag%20Handle%20Structure))
  (bind _bagtype (Utilities|Struct|BreakSBZBagHandle Handle))
  (bind _bagmidmap (Variables|Default|GetBagMIDMap))
  (bind _value (Utilities|Map|Find _bagmidmap _bagtype))
  (bind _outactors (Actor|GetAllActorsOfClass "/Game/Prototype/Blueprints/Bags/BP_BaseBagSecured.BP_BaseBagSecured_C"))
  (if (not (== (Rendering|Material|GetMaterial (Variables|/Game/Prototype/Blueprints/Bags/BP_BaseBagSecured.BP_BaseBagSecured_C|GetStaticMesh (Utilities|Array|Get(acopy) _outactors (Variables|Default|GetSecureIndex))) 0) _value))
    (Rendering|Material|SetMaterial (Variables|/Game/Prototype/Blueprints/Bags/BP_BaseBagSecured.BP_BaseBagSecured_C|GetStaticMesh (Utilities|Array|Get(acopy) _outactors (Variables|Default|GetSecureIndex))) 0 _value)
    (Math|Integer|IncrementInt (Variables|Default|GetSecureIndex))))

(event EventBeginPlay
  (bind _bagtexturemap (Variables|Default|GetBagTextureMap))
  (bind _objectinstance (CallFunction|FindPersistentModObjectbyClass "/Game/Mods/_NadzMods/BagMod/BP_UniqueLootBag_Pers.BP_UniqueLootBag_Pers_C"))
  (Variables|Default|SetMyPersistentManagerObject _objectinstance)
  (bind _keys (Utilities|Map|Keys _bagtexturemap))
  (for _array_element _keys
    (bind _returnvalue (Rendering|Material|CreateDynamicMaterialInstance "/Game/Mods/_NadzMods/BagMod/MI_CustomBag.MI_CustomBag" (Utilities|String|StringToName (Utilities|String|Append "MID_" (Utilities|String|ToString(Text) (Variables|/Script/Starbreeze.SBZCarryType|GetCarryName _array_element)))) "None" :!class /Script/Engine.KismetMaterialLibrary))
    (Rendering|Material|SetTextureParameterValue _returnvalue "Base Color" (.Value (Utilities|Map|Find _bagtexturemap _array_element)))
    (Utilities|Map|Add (Variables|Default|GetBagMIDMap) _array_element _returnvalue)
    (bind _outactors (Actor|GetAllActorsOfClass "/Script/Starbreeze.SBZBagTriggerVolume"))
    (for _array_element_2 _outactors
      (EventDispatchers|AssignOnBagEnteredorSecured _array_element_2 (delegate Custom|OnBagEnteredOrSecured_Event_0)))))

(event Collision|EventActorBeginOverlap
  (params (OtherActor :type Actor%20Object%20Reference))
  (|CallParentFunction OtherActor) ; This node is disabled and will not be called.\nDrag off pins to build functionality.
)

(event EventTick
  (params (DeltaSeconds :type Float%20%28single-precision%29))
  (Utilities|FlowControl|Sequence
    (:then_0
      (bind _outactors (Actor|GetAllActorsOfClass "/Game/Prototype/Blueprints/Bags/BP_BaseValuableBag.BP_BaseValuableBag_C"))
      (bind _array_element (Utilities|Array|ForEachLoopwithBreak _outactors)
        (:LoopBody
          (for _array_element_2 (Actor|GetComponentsByClass _array_element "/Script/Engine.StaticMeshComponent")
            (if (not (== (Rendering|Material|GetMaterial _array_element_2 0) (.Value (Utilities|Map|Find (Variables|Default|GetBagMIDMap) (.BagType (Utilities|Struct|BreakSBZBagHandle (Variables|/Script/Starbreeze.SBZBagItem|GetBag _array_element)))))))
              (Rendering|Material|SetMaterial _array_element_2 0 (.Value (Utilities|Map|Find (Variables|Default|GetBagMIDMap) (.BagType (Utilities|Struct|BreakSBZBagHandle (Variables|/Script/Starbreeze.SBZBagItem|GetBag _array_element)))))))))))
    (:then_1
      (bind _outactors_2 (Actor|GetAllActorsOfClass "/Game/Prototype/Blueprints/Bags/BP_BackItemBagBase.BP_BackItemBagBase_C"))
      (bind _array_element_3 (Utilities|Array|ForEachLoopwithBreak _outactors_2)
        (:LoopBody
          (if (not (== (Rendering|Material|GetMaterial (Variables|/Script/Starbreeze.SBZCarriedBag|GetSkeletalMeshComponentBudgeted _array_element_3) 0) (.Value (Utilities|Map|Find (Variables|Default|GetBagMIDMap) (.BagType (Utilities|Struct|BreakSBZBagHandle (Variables|/Script/Starbreeze.SBZCarriedBag|GetBagHandle _array_element_3)))))))
            (Rendering|Material|SetMaterial (Variables|/Script/Starbreeze.SBZCarriedBag|GetSkeletalMeshComponentBudgeted _array_element_3) 0 (.Value (Utilities|Map|Find (Variables|Default|GetBagMIDMap) (.BagType (Utilities|Struct|BreakSBZBagHandle (Variables|/Script/Starbreeze.SBZCarriedBag|GetBagHandle _array_element_3))))))))))))

(fn ConstructionScript)